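; Sante is a health pickup that heals the player's Character_Controller when it overlaps the Box component, then destroys itself.
; The overlap handler loops over every Sante actor in the level, hiding each one's BouteilleDeSoinText.
; Each iteration also adds a fixed, clamped amount of health, plays the Soin sound and calls DestroyActor on self, so the heal repeats per Sante instance found.
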(event OnComponentBeginOverlap(Box)
  (params (OverlappedComponent :type Primitive%20Component%20Object%20Reference) (OtherActor :type Actor%20Object%20Reference) (OtherComp :type Primitive%20Component%20Object%20Reference) (OtherBodyIndex :type Integer) (bFromSweep :type Boolean) (SweepResult :type Hit%20Result%20Structure%20%28by%20ref%29))
  ;[1 1 1] Si le joueur touche l'acteur "Sante"...
  (bind _ascharacter_controller (Utilities|Casting|CastToCharacter_Controller OtherActor))
  ;;[1 1 1] On cherche tous les acteurs qui s'appelle "Sante"
  (bind _outactors (Actor|GetAllActorsOfClass "Sante_C"))
  (for _array_element _outactors
    ;;[1 1 1] On cache le texte par-dessus l'acteur "Sante"
    (Development|SetHiddeninGame (Variables|Sante_C|GetBouteille%20de%20soin%20-%20Text _array_element) true false)
    ;;[1 1 1] On ajoute 20 vies à la santé du joueur
    (Variables|/Game/Blueprints/Character_Controller.Character_Controller_C|SetSante _ascharacter_controller (Math|Float|Clamp(Float) (+ (Variables|/Game/Blueprints/Character_Controller.Character_Controller_C|GetSante _ascharacter_controller) 2e+01) 0.0 1e+02))
    ;;[1 1 1] On joue le son de la santé et on détruit l'acteur "Sante"
    (Audio|PlaySound2D "/Game/EffetsSonores/Soin.Soin" 1.0 1.0 0.0 0 0)
    (Actor|DestroyActor)))

(fn ConstructionScript)