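; Couteau is a knife hazard that takes 10 health from the player on contact and plays a damage sound.
; Its capsule overlap casts to Character_Controller and lowers the clamped Sante value.
; PeuxPrendreDuDommage gates damage: an overlap clears it before the cast, and only a later overlap sets it again, without dealing damage.
; The closing one-second Delay leads to nothing, so it provides no cooldown.
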(event OnComponentBeginOverlap(Capsule)
  (params (OverlappedComponent :type Primitive%20Component%20Object%20Reference) (OtherActor :type Actor%20Object%20Reference) (OtherComp :type Primitive%20Component%20Object%20Reference) (OtherBodyIndex :type Integer) (bFromSweep :type Boolean) (SweepResult :type Hit%20Result%20Structure%20%28by%20ref%29))
  ;[1 1 1] Si le joueur touche le couteau, il perd 10 vies et on fait joueur le son de dommage
  (if (Variables|Default|GetPeuxPrendreDuDommage)
    (Variables|Default|SetPeuxPrendreDuDommage false)
    (bind _ascharacter_controller (Utilities|Casting|CastToCharacter_Controller OtherActor))
    (Variables|/Game/Blueprints/Character_Controller.Character_Controller_C|SetSante _ascharacter_controller (Math|Float|Clamp(Float) (- (Variables|/Game/Blueprints/Character_Controller.Character_Controller_C|GetSante _ascharacter_controller) 1e+01) 0.0 1e+02))
    (Audio|PlaySound2D "/Game/EffetsSonores/Dommage.Dommage" 1.0 1.0 0.0 0 0)
    (Utilities|FlowControl|Delay 1.0)
    (else
      (Variables|Default|SetPeuxPrendreDuDommage true))))

(event EventBeginPlay)

(event Collision|EventActorBeginOverlap
  (params (OtherActor :type Actor%20Object%20Reference)))

(event EventTick
  (params (DeltaSeconds :type Float%20%28single-precision%29)))

(fn ConstructionScript)