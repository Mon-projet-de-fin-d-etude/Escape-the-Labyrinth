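; Player character Blueprint handling movement, health and pausing.
; Input axes drive capsule-relative movement and camera look, alongside jumping and a Vitesse event that sets walk speed.
; BeginPlay shows the Sante widget; damage, self-inflicted with N for apparent testing, lowers clamped health and prints it or a death message.
; Pause opens the MenuPause widget, shows the cursor, switches to UI-only input and pauses the game.
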(event Custom|Vitesse
  (params (Vitesse :type Float%20%28double-precision%29))
  (Variables|/Script/Engine.CharacterMovementComponent|SetMaxWalkSpeed (Variables|Character|GetCharacterMovement) Vitesse))

(event EventBeginPlay
  (bind _returnvalue (UserInterface|CreateWidget "/Game/UI/Sante.Sante_C" (Game|GetPlayerController 0)))
  (UserInterface|Viewport|AddtoViewport _returnvalue 0))

(event Collision|EventActorBeginOverlap
  (params (OtherActor :type Actor%20Object%20Reference)))

(event EventTick
  (params (DeltaSeconds :type Float%20%28single-precision%29)))

(event Game|Damage|EventAnyDamage
  (params (Damage :type Float%20%28single-precision%29) (DamageType :type Damage%20Type%20Object%20Reference) (InstigatedBy :type Controller%20Object%20Reference) (DamageCauser :type Actor%20Object%20Reference))
  (Variables|Default|SetSante (Math|Float|Clamp(Float) (- (Variables|Default|GetSante) Damage) 0.0 1e+02))
  (if (<= (Variables|Default|GetSante) 0.0)
    (Development|PrintString "Mort!!!")
    (else
      (Development|PrintString (Utilities|String|ToString(Float) (Variables|Default|GetSante))))))

(event Input|ActionEvents|InputActionJump
  (params (Key :type Key%20Structure :default "None"))
  (:Pressed
    (Character|Jump)))

(event Input|ActionEvents|InputActionPause
  (params (Key :type Key%20Structure :default "None"))
  (bind _returnvalue (Game|GetPlayerController 0))
  (:Pressed
    (bind _returnvalue_2 (UserInterface|CreateWidget "/Game/UI/MenuPause.MenuPause_C"))
    (UserInterface|Viewport|AddtoViewport _returnvalue_2 0)
    (Variables|/Script/Engine.PlayerController|SetbShowMouseCursor _returnvalue true)
    (Input|SetInputModeUIOnly _returnvalue 0 "DoNotLock" false)
    (Game|SetGamePaused true)))

(event Input|AxisEvents|InputAxisTourner
  (params (AxisValue :type Float%20%28single-precision%29))
  (Pawn|Input|AddControllerYawInput AxisValue))

(event Input|AxisEvents|InputAxisRegarderenhaut
  (params (AxisValue :type Float%20%28single-precision%29))
  (Pawn|Input|AddControllerPitchInput AxisValue))

(event Input|AxisEvents|InputAxisAvance
  (params (AxisValue :type Float%20%28single-precision%29))
  (Pawn|Input|AddMovementInput (Math|Vector|GetForwardVector (Variables|Collision|GetCapsuleComponent)) AxisValue false))

(event Input|AxisEvents|InputAxisCôtés
  (params (AxisValue :type Float%20%28single-precision%29))
  (Pawn|Input|AddMovementInput (Math|Vector|GetRightVector (Variables|Collision|GetCapsuleComponent)) AxisValue false))

(event Input|KeyboardEvents|N
  (params (Key :type Key%20Structure :default "None"))
  (:Pressed
    (Game|Damage|ApplyDamage self 1e+01 0 0)))

(fn ConstructionScript)