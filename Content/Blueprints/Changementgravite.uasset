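; Changementgravite is a pickup actor that temporarily halves the gravity scale of the Character_Controller that touches it.
; On box overlap, it loops over all Changementgravite actors to hide their text, disabling its own collision and hiding itself within that loop.
; A five-second Delay, also inside the loop, precedes restoring normal gravity and destroying the touched actor.
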(event OnComponentBeginOverlap(Box)
  (params (OverlappedComponent :type Primitive%20Component%20Object%20Reference) (OtherActor :type Actor%20Object%20Reference) (OtherComp :type Primitive%20Component%20Object%20Reference) (OtherBodyIndex :type Integer) (bFromSweep :type Boolean) (SweepResult :type Hit%20Result%20Structure%20%28by%20ref%29))
  ;[1 1 1] Si le joueur touche l'acteur "Changement de gravité"...
  (bind _ascharacter_controller (Utilities|Casting|CastToCharacter_Controller OtherActor))
  ;;[1 1 1] On cherche tous les acteurs qui sont de type "Changement de gravité"
  (bind _outactors (Actor|GetAllActorsOfClass "Changementgravite_C"))
  (for _array_element _outactors
    ;;[1 1 1] On cache le texte de l'acteur "Changement de gravité" et on cache l'acteur "Changemendt de gravité"
    (Development|SetHiddeninGame (Variables|Changementgravite_C|GetChangement%20de%20gravité%20-%20Text _array_element) true false)
    (Collision|SetCollisionEnabled (Variables|Default|GetBox) "NoCollision")
    (Rendering|SetActorHiddenInGame true)
    ;[1 1 1] La gravité devient plus légère, car on divise la gravité du jeu en 2 (de 1 à 0.5). Après 5 secondes, la gravité revient à sa normale et on détruit l'acteur de changement de gravité
    (Variables|/Script/Engine.CharacterMovementComponent|SetGravityScale (Variables|/Script/Engine.Character|GetCharacterMovement _ascharacter_controller) 0.5)
    (Utilities|FlowControl|Delay 5.0)
    (Variables|/Script/Engine.CharacterMovementComponent|SetGravityScale (Variables|/Script/Engine.Character|GetCharacterMovement _ascharacter_controller) 1.0)
    (Actor|DestroyActor)))

(fn ConstructionScript)