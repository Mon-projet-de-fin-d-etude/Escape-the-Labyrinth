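; BP_Roche is a rock hazard that hurts the player on contact and destroys itself 10 seconds after spawning.
; Overlapping its Sphere with a Character_Controller lowers that character's Sante by a fixed, clamped amount and plays a damage sound.
; The hit also plays the SangFrappe blood-hit widget animation, creating the widget on first use and reusing it for that rock.
; The rock is not destroyed on impact.
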(event OnComponentBeginOverlap(Sphere)
  (params (OverlappedComponent :type Primitive%20Component%20Object%20Reference) (OtherActor :type Actor%20Object%20Reference) (OtherComp :type Primitive%20Component%20Object%20Reference) (OtherBodyIndex :type Integer) (bFromSweep :type Boolean) (SweepResult :type Hit%20Result%20Structure%20%28by%20ref%29))
  ;[1 1 1] Si le joueur se fait frapper par une roche, il perd 15 vies.
  (bind _ascharacter_controller (Utilities|Casting|CastToCharacter_Controller OtherActor))
  (Variables|/Game/Blueprints/Character_Controller.Character_Controller_C|SetSante _ascharacter_controller (Math|Float|Clamp(Float) (- (Variables|/Game/Blueprints/Character_Controller.Character_Controller_C|GetSante _ascharacter_controller) 15.0) 0.0 1e+02))
  (Audio|PlaySound2D "/Game/Son-Musique/EffetsSonores/Dommage.Dommage" 1.0 1.0 0.0 0 0)
  (Variables|Default|GetSangFrappe
    (:then
      (Default|JouerAnimationFrappe (Variables|Default|GetSangFrappe)))
    (:else
      (bind _returnvalue (UserInterface|CreateWidget "/Game/Blueprints-UI/Sang.Sang_C" (Game|GetPlayerController 0)))
      (bind _output_get (Variables|Default|SetSangFrappe _returnvalue))
      (UserInterface|Viewport|AddtoViewport (Variables|Default|GetSangFrappe) 0)
      (Default|JouerAnimationFrappe (Variables|Default|GetSangFrappe)))))

(event EventBeginPlay
  ;[1 1 1] Après 10 secondes, la roche se fait détruire par elle même
  (Utilities|FlowControl|Delay 1e+01)
  (Actor|DestroyActor))

(fn ConstructionScript)